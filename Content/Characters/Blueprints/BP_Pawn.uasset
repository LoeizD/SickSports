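; Player pawn for a multiplayer bike arena game where riders bat props at one another to score toward a win.
; Axis input drives movement and look, feeding FMOD-style engine sound parameters, while a BP_Rider handles bat charge, swing and score display.
; The authority assigns color and name, stuns players hit by others' props and credits the prop's owner.
; Wall hits trace-teleport the pawn onto the new wall, briefly disabling collision; reorientation code is disconnected.
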(event OnComponentBeginOverlap(Capsule)
  (params (OverlappedComponent :type Primitive%20Component%20Object%20Reference) (OtherActor :type Actor%20Object%20Reference) (OtherComp :type Primitive%20Component%20Object%20Reference) (OtherBodyIndex :type Integer) (bFromSweep :type Boolean) (SweepResult :type Hit%20Result%20Structure%20%28by%20ref%29))
  (bind _returnvalue (Transformation|GetActorTransform))
  (Networking|SwitchHasAuthority
    (:Authority
      (if (not (Variables|Default|GetStun))
        (if (Variables|Default|GetPlayerIsReady)
          (bind _asbp_props_parent (Utilities|Casting|CastToBP_Props_Parent OtherActor))
          (if (Variables|/Game/Props/BP_Props_Parent.BP_Props_Parent_C|GetIsPunched _asbp_props_parent)
            (if (!= self (Variables|/Game/Props/BP_Props_Parent.BP_Props_Parent_C|GetMyOwnerPlayer _asbp_props_parent)) ; Si touché par un objet qui n'est pas à moi
              (Utilities|FlowControl|Sequence
                (:then_0
                  ;[1 1 1] Stun
                  (Variables|Default|SetStun true)
                  (CallFunction|OwnerCamShakeHit)
                  (Utilities|FlowControl|Delay 0.7)
                  (Variables|Default|SetStun false))
                (:then_1
                  ;[1 1 1] Comment
                  (bind _asbp_pawn (Utilities|Casting|CastToBP_Pawn (Variables|/Game/Props/BP_Props_Parent.BP_Props_Parent_C|GetMyOwnerPlayer _asbp_props_parent)))
                  (CallFunction|MulticastAddScore _asbp_pawn))
                (:then_2
                  ;[1 1 1] SOUND
                  (Class|FMODAudioComponent|Play (Variables|Default|GetHitSound))
                  (Utilities|FlowControl|Delay (Math|Random|RandomFloatinRange 0.03 0.2))
                  (Class|FMODAudioComponent|Play (Variables|Default|GetHitVoice)))
                (:then_3
                  (Rendering|Material|SetVectorParameterValue "/Game/InfinityBladeEffects/MPC_All.MPC_All" "TempColor" (Variables|BP_Pawn_C|GetMyColor (.AsBP%20Pawn (Utilities|Casting|CastToBP_Pawn (Variables|/Game/Props/BP_Props_Parent.BP_Props_Parent_C|GetMyOwnerPlayer _asbp_props_parent)))) :!class /Script/Engine.KismetMaterialLibrary)
                  (bind _returnvalue_2 (Effects|SpawnEmitteratLocation "/Game/InfinityBladeEffects/Effects/FX_Ambient/Fire/P_LavaFire_PourBase.P_LavaFire_PourBase" (.location _returnvalue) (.rotation _returnvalue)))
                  (Transformation|SetWorldScale3D _returnvalue_2 "5.000000,5.000000,5.000000"))))))))))

(event Custom|UpdateTransform
  (params (NewParam :type Transform))
  (CallFunction|UpdateMyTransform NewParam))

(event Custom|Multicast_AddScore
  ;[1 1 1] Comment
  (CallFunction|AddScore))

(event Custom|ServerPunch
  (params (PunchedProps :type Actor%20Object%20Reference) (PuncherForwardVector :type Vector) (AddedForce :type Float%20%28single-precision%29) (PlayerCurrentFloor :type Actor%20Object%20Reference) (PlayerColor :type Linear%20Color%20Structure) (OwnerPlayer :type Actor%20Object%20Reference))
  (bind _asbp_props_parent (Utilities|Casting|CastToBP_Props_Parent PunchedProps))
  (Default|Punched _asbp_props_parent PuncherForwardVector AddedForce PlayerCurrentFloor PlayerColor OwnerPlayer))

(event Custom|SendTransformToAllPlayers
  ;[1 0.8706 0] Ce n'est même pas utilisé en fait non ?  ... LOOOOL
  (CallFunction|UpdateTransform (Transformation|GetActorTransform)))

(event Custom|Owning_HitWall
  (params (Object :type Object%20Object%20Reference))
  (bind _asbp_wall (Utilities|Casting|CastToBP_Wall Object))
  (CallFunction|WallRide _asbp_wall))

(event Custom|EngineSOund
  (bind _sfxengine (Variables|Default|GetSfxEngine))
  ;[1 1 1] EngineSound
  (CallFunction|SfxTimer)
  (if (and (== (Input|AxisValues|GetForward) 0.0) (== (Input|AxisValues|GetStrafe) 0.0))
    (Variables|Default|SetTimerSoundSet false)
    (Class|FMODAudioComponent|SetParameter _sfxengine "LOAD" -1.0)
    (Class|FMODAudioComponent|SetParameter _sfxengine "PD" 1.0)
    (Class|FMODAudioComponent|SetParameter _sfxengine "SKID" 0.0)
    (Variables|Default|SetLOADEngineSound true)
    (if (>= (Variables|Default|GetBrakeTimer) 0.3)
      (Class|FMODAudioComponent|SetParameter _sfxengine "BP" 1.0)
      (goto _label Reset)
      (else
        (goto _label Reset)))
    (else
      (Variables|Default|SetTimerSoundSet true)
      (if (and (== (Input|AxisValues|GetForward) 0.0) (!= (Input|AxisValues|GetStrafe) 0.0))
        (Class|FMODAudioComponent|SetParameter _sfxengine "SKID" 1.0)
        (else
          (Class|FMODAudioComponent|SetParameter _sfxengine "SKID" 0.0)))
      (Class|FMODAudioComponent|SetParameter _sfxengine "BP" 0.0)
      (Utilities|FlowControl|MultiGate false false -1 :!label _label
        (:Out%200
          (Class|FMODAudioComponent|SetParameter _sfxengine "LOAD" 1.0)
          (Class|FMODAudioComponent|SetParameter _sfxengine "PD" 0.0)
          (Variables|Default|SetLOADEngineSound false))
        (:Out%201
          (Utilities|FlowControl|Delay 0.2)
          (if (not (Variables|Default|GetLOADEngineSound))
            (Class|FMODAudioComponent|SetParameter _sfxengine "LOAD" 0.0)))))))

(event Custom|OwnerCamShakeHit
  ;[1 1 1] Stun
  (Class|PlayerController|ClientPlayCameraShake (Game|GetPlayerController 0) "/Game/Characters/Blueprints/CS_Hit.CS_Hit_C" 1.0 "CameraLocal" "0, 0, 0"))

(event Custom|InitHonk
  (Variables|Default|SetKlaxonPlayed 0))

(event EventTick
  (params (DeltaSeconds :type Float%20%28single-precision%29))
  ;[0.4416 1 0] Event Tick
  (Utilities|FlowControl|Sequence
    (:then_0
      (CallFunction|EngineSOund)
      (Variables|Movement|SetForward (Input|AxisValues|GetForward))
      (Variables|Movement|SetLeft (* (Input|AxisValues|GetStrafe) -1.0))
      (Variables|Movement|SetLook (Input|AxisValues|GetMouseRight))
      (CallFunction|ClampActorLocation))
    (:then_1
      ;[1 1 1] Reset col secu
      (if (!= (Variables|WallHit|GetOneTestAtTimeSecu) 0)
        (bind _output_get (Variables|WallHit|SetOneTestAtTimeSecu (- (Variables|WallHit|GetOneTestAtTimeSecu) 1)))
        (if (== _output_get 0)
          (Collision|SetActorEnableCollision true))))))

(event EventBeginPlay
  (bind _returnvalue (Transformation|GetActorUpVector))
  (bind _returnvalue_2 (Transformation|GetActorLocation))
  ;[0.06855 1 0] Begin Play
  (Utilities|FlowControl|Sequence
    (:then_0
      (CallFunction|InitEngineSound)
      ;[1 1 1] REF GameInstance
      (Variables|Default|SetGameInstanceREF (.AsBP%20Game%20Instance (Utilities|Casting|CastToBP_GameInstance (Game|GetGameInstance))))
      ;[1 1 1] REF Gamemode
      (Variables|Default|SetGamemodeREF (.AsBP%20Gamemode (Utilities|Casting|CastToBP_Gamemode (Game|GetGameMode))))
      (Utilities|FlowControl|Sequence
        (:then_0
          ;[0.5568 0 1] server
          (Networking|SwitchHasAuthority
            (:Authority
              (CallFunction|AddMetoListOfPawns)
              ;[1 1 1] Get color
              (bind _output_get (Variables|Default|SetMyColor (Utilities|Array|Get(acopy) (Variables|/Game/Base/Blueprint/BP_Gamemode.BP_Gamemode_C|GetColors (.AsBP%20Gamemode (Utilities|Casting|CastToBP_Gamemode (Game|GetGameMode)))) (Utilities|Array|FindItem (Variables|/Game/Base/Blueprint/BP_GameInstance.BP_GameInstance_C|GetServerListOfPawns (Variables|Default|GetGameInstanceREF)) self))))
              ;[1 1 1] Get name
              (bind _output_get_2 (Variables|Default|SetMyName (Utilities|Array|Get(acopy) (Variables|/Game/Base/Blueprint/BP_Gamemode.BP_Gamemode_C|GetColorsNames (.AsBP%20Gamemode (Utilities|Casting|CastToBP_Gamemode (Game|GetGameMode)))) (Utilities|Array|FindItem (Variables|/Game/Base/Blueprint/BP_GameInstance.BP_GameInstance_C|GetServerListOfPawns (Variables|Default|GetGameInstanceREF)) self))))
              ;[1 0 0] DELAY
              (Utilities|FlowControl|Delay 1.0)
              (bind (_outhit _returnvalue_3) (Collision|LineTraceForObjects (+ _returnvalue_2 (* _returnvalue 2e+01)) (+ _returnvalue_2 (* _returnvalue -2e+02)) (Utilities|Array|MakeArray "ObjectTypeQuery8") false 0 "None"))
              (if _returnvalue_3
                (bind _output_get_3 (Variables|Default|SetCurrentFloor (.HitActor (Collision|BreakHitResult _outhit))))
                (Variables|WallHit|SetCurrentWall (.HitActor (Collision|BreakHitResult _outhit)))
                (Variables|WallHit|SetPreviousWall (.HitActor (Collision|BreakHitResult _outhit)))
                (Variables|Default|SetPlayerIsReady true)))))
        (:then_1
          ;[1 0.4217 0] Dynamic Child Actor
          (CallFunction|SpawnBikeVisual))))
    (:then_1
      (Utilities|Time|SetTimerbyEvent (delegate Custom|SendTransformToAllPlayers) 0.05 true)
      (CallFunction|SaveAllWallsinVariables)
      (Class|SceneComponent|DetachfromParent (Variables|Default|GetRepereMur) false true))))

(event Input|ActionEvents|InputActionPunch
  (params (Key :type Key%20Structure :default "AnyKey"))
  (bind _battecol (Variables|Default|GetBatteCol))
  (bind _riderref (Variables|Default|GetRiderRef))
  (bind _overlappingactors (Collision|GetOverlappingActors _battecol "/Game/Props/BP_Props_Parent.BP_Props_Parent_C" :!class /Script/Engine.PrimitiveComponent))
  (bind _returnvalue (Utilities|Array|Length _overlappingactors))
  (bind _returnvalue_2 (> _returnvalue 0))
  (:Pressed
    (Utilities|IfNotStunned
      (:NotStunned
        (Default|Charge _riderref))))
  (:Released
    (Utilities|IfNotStunned
      (:NotStunned
        (Default|Hit _riderref)
        (CallFunction|PunchF _returnvalue_2)
        ;[1 1 1] Batte test collision
        (if _returnvalue_2
          (for _array_element _overlappingactors
            (Utilities|FlowControl|Sequence
              (:then_0
                (Rendering|Material|SetVectorParameterValue "/Game/InfinityBladeEffects/MPC_All.MPC_All" "TempColor" (Variables|Default|GetMyColor) :!class /Script/Engine.KismetMaterialLibrary)
                (Effects|SpawnEmitteratLocation "/Game/InfinityBladeEffects/Effects/FX_Ambient/Fire/P_LavaFire_PourBase.P_LavaFire_PourBase" (.location (Transformation|GetActorTransform _array_element)) (.rotation (Transformation|GetActorTransform _array_element))))
              (:then_1
                ;[1 1 1] Punch Props
                (CallFunction|ServerPunch _array_element (Transformation|GetActorForwardVector) (Variables|Default|GetPunchForce) (Variables|Default|GetCurrentFloor) (Variables|Default|GetMyColor) self)))))))))

(event Input|ActionEvents|InputActionKlaxon
  (params (Key :type Key%20Structure :default "AnyKey"))
  (:Pressed
    (CallFunction|Klaxon)
    (Utilities|Time|SetTimerbyEvent (delegate Custom|InitHonk) 1.0)))

(event Input|AxisEvents|InputAxisForward
  (params (AxisValue :type Float%20%28single-precision%29))
  (Utilities|IfNotStunned
    (:NotStunned
      (Transformation|AddActorLocalOffset (Math|Vector|MakeVector (* AxisValue (* (Variables|Default|GetForwardSpeed) (Utilities|Time|GetWorldDeltaSeconds))) 0.0 0.0) false false))))

(event Input|AxisEvents|InputAxisStrafe
  (params (AxisValue :type Float%20%28single-precision%29))
  (Utilities|IfNotStunned
    (:NotStunned
      (Transformation|AddActorLocalOffset (Math|Vector|MakeVector 0.0 (* AxisValue (* (Variables|Default|GetForwardSpeed) (Utilities|Time|GetWorldDeltaSeconds))) 0.0) false false))))

(event Input|AxisEvents|InputAxisMouseUp
  (params (AxisValue :type Float%20%28single-precision%29))
  (bind _cameraanchor (Variables|Default|GetCameraAnchor))
  (Utilities|IfNotStunned
    (:NotStunned
      (Transformation|SetRelativeRotation _cameraanchor (Math|Rotator|MakeRotator 0.0 (Math|Float|Clamp(Float) (+ (.pitch (Variables|/Script/Engine.SceneComponent|GetRelativeRotation _cameraanchor)) (* AxisValue (* (Variables|Default|GetMouseSpeed) (Utilities|Time|GetWorldDeltaSeconds)))) -85.0 85.0) 0.0) false false))))

(event Input|AxisEvents|InputAxisMouseRight
  (params (AxisValue :type Float%20%28single-precision%29))
  (Utilities|IfNotStunned
    (:NotStunned
      (Transformation|AddActorLocalRotation (Math|Rotator|MakeRotator 0.0 0.0 (* AxisValue (* (Variables|Default|GetMouseSpeed) (Utilities|Time|GetWorldDeltaSeconds)))) false false))))

(event Input|KeyboardEvents|Escape
  (params (Key :type Key%20Structure :default "AnyKey"))
  (:Pressed
    (Development|ExecuteConsoleCommand "Exit")))

(fn ConstructionScript)

(fn UpdateMyTransform
  (params (NewTransform :type Transform%20%28by%20ref%29))
  (Transformation|SetActorTransform NewTransform))

(fn InitEngineSound
  (bind _sfxengine (Variables|Default|GetSfxEngine))
  (Class|FMODAudioComponent|Play _sfxengine)
  (Class|FMODAudioComponent|SetParameter _sfxengine "LOAD" -1.0))

(fn SfxTimer
  (if (Variables|Default|GetTimerSoundSet)
    (Variables|Default|SetBrakeTimer (+ (Variables|Default|GetBrakeTimer) (Utilities|Time|GetWorldDeltaSeconds)))
    (else
      (Variables|Default|SetBrakeTimer 0.0))))

(fn OnRepMyColor)

(fn AddScore
  (bind _gameinstanceref (Variables|Default|GetGameInstanceREF))
  (CallFunction|PointSound)
  ;[1 1 1] Add Score
  (bind _output_get (Variables|Default|SetCurrentScore (+ (Variables|Default|GetCurrentScore) 1)))
  ;[1 1 1] Update Score on bike
  (Default|UpdateScore (Variables|Default|GetRiderRef) _output_get)
  (CallFunction|WinSong)
  (if (>= (Variables|Default|GetCurrentScore) (Variables|/Game/Base/Blueprint/BP_GameInstance.BP_GameInstance_C|GetPointsToWin _gameinstanceref)) ; If enough points to Win
    (Default|Winner _gameinstanceref (Variables|Default|GetMyColor) (Variables|Default|GetMyName))))

(fn AddMetoListOfPawns
  (Utilities|Array|Add (Variables|/Game/Base/Blueprint/BP_GameInstance.BP_GameInstance_C|GetServerListOfPawns (Variables|Default|GetGameInstanceREF)) self))

(fn Klaxon
  (Class|FMODAudioComponent|Play (Variables|Default|GetKlax))
  (Variables|Default|SetKlaxonPlayed (+ (Variables|Default|GetKlaxonPlayed) 1))
  (if (and (== (Math|Integer|%(Integer) (Variables|Default|GetKlaxonPlayed) 10) 0) (!= (Variables|Default|GetKlaxonPlayed) 0))
    (bind _outactors (Actor|GetAllActorsOfClass "/Game/Sound/BP_SoundManager.BP_SoundManager_C"))
    (Default|EyesOfTiger _outactors)))

(fn PunchF
  (params (Hit :type Boolean))
  (bind _punchsound (Variables|Default|GetPunchSound))
  (if Hit
    (Variables|Default|SetHitParam 1.0)
    (else
      (Variables|Default|SetHitParam 0.0)))
  (Class|FMODAudioComponent|SetParameter _punchsound "PUNCH" (Variables|Default|GetHitParam))
  (Class|FMODAudioComponent|Play _punchsound))

(fn WinSong
  (bind _outactors (Actor|GetAllActorsOfClass "/Game/Sound/BP_SoundManager.BP_SoundManager_C"))
  (Default|WinSong _outactors (Variables|Default|GetCurrentScore)))

(fn PointSound
  (Class|FMODAudioComponent|Play (Variables|Default|GetPoint))
  (bind _outactors (Actor|GetAllActorsOfClass "/Game/Sound/BP_Mentions.BP_Mentions_C"))
  (Default|PointScore _outactors))

(fn SpawnBikeVisual
  (bind _returnvalue (Game|SpawnActorfromClass "/Game/Coco/Moto/BP_Rider.BP_Rider_C" (Math|Transform|MakeTransform "0, 0, 0" "0,0.000000, 0" "1,1,1") "Undefined" 0 self 0))
  (Variables|Default|SetRiderRef _returnvalue))

(fn CreateAddOfWallstoIgnore
  (Utilities|Array|Clear (Variables|WallHit|GetWallsToIgnore))
  (bind _outactors (Actor|GetAllActorsOfClass "/Game/Room/BP_Wall.BP_Wall_C"))
  (for _array_element _outactors
    (if (!= _array_element (Variables|WallHit|GetCurrentWall)) ; Si est n'importe quel wall\nsauf le wall qu'on collisionne\nsur lequel on a envie de grimper
      (Utilities|Array|Add (Variables|WallHit|GetWallsToIgnore) _array_element))))

(fn WallRide
  (params (HitWall :type BP%20Wall%20Object%20Reference))
  (bind _arrow (Variables|Default|GetArrow))
  (Variables|WallHit|SetHitWall HitWall)
  ;[1 1 1] Test si c'est bien un nouveau wall
  (if (!= (Variables|WallHit|GetHitWall) (Variables|WallHit|GetCurrentWall))
    (if (== (Variables|WallHit|GetOneTestAtTimeSecu) 0)
      (CallFunction|AddSecuWallandDeactivateColl)
      ;[1 1 1] useless?
      (Variables|WallHit|SetPREPreviousWall (Variables|WallHit|GetPreviousWall))
      (Variables|WallHit|SetPreviousWall (Variables|WallHit|GetCurrentWall))
      (Variables|WallHit|SetCurrentWall (Variables|WallHit|GetHitWall))
      (Variables|WallHit|SetLTNormal (Math|Vector|GetForwardVector (Variables|/Game/Room/BP_Wall.BP_Wall_C|GetWallUp (Variables|WallHit|GetHitWall))))
      (CallFunction|CreateAddOfWallstoIgnore)
      (bind (_outhit _returnvalue) (Collision|LineTraceForObjects (+ (Transformation|GetWorldLocation _arrow) (* (Math|Vector|GetForwardVector _arrow) -3e+04)) (+ (Transformation|GetWorldLocation _arrow) (* (Math|Vector|GetForwardVector _arrow) 2e+03)) (Utilities|Array|MakeArray "ObjectTypeQuery8") false (Variables|WallHit|GetWallsToIgnore) "Persistent"))
      (if _returnvalue
        (Transformation|SetActorLocation (.ImpactPoint (Collision|BreakHitResult _outhit)) false false)
        (if (== (Variables|WallHit|GetPreviousWall) (Variables|WallHit|GetWall_Kart))
          (Development|PrintString "Kart")
          (elif (== (Variables|WallHit|GetPreviousWall) (Variables|WallHit|GetWall_Judo))
            (Development|PrintString "Judo")
            (elif (== (Variables|WallHit|GetPreviousWall) (Variables|WallHit|GetWall_Basket))
              (Development|PrintString "Basket")
              (elif (== (Variables|WallHit|GetPreviousWall) (Variables|WallHit|GetWall_Tennis))
                (Development|PrintString "Tennis")
                (elif (== (Variables|WallHit|GetPreviousWall) (Variables|WallHit|GetWall_Trackfield))
                  (Development|PrintString "Trackfield")
                  (elif (== (Variables|WallHit|GetPreviousWall) (Variables|WallHit|GetWall_Gym))
                    (Development|PrintString "Gym")
                    (if (== (Variables|WallHit|GetHitWall) (Variables|WallHit|GetWall_Kart))
                      (Development|PrintString "Kart")
                      (elif (== (Variables|WallHit|GetHitWall) (Variables|WallHit|GetWall_Judo))
                        (Development|PrintString "Judo")
                        (elif (== (Variables|WallHit|GetHitWall) (Variables|WallHit|GetWall_Basket))
                          (Development|PrintString "Basket")
                          (elif (== (Variables|WallHit|GetHitWall) (Variables|WallHit|GetWall_Tennis))
                            (Development|PrintString "Tennis")
                            (elif (== (Variables|WallHit|GetHitWall) (Variables|WallHit|GetWall_Trackfield))
                              (Development|PrintString "Trackfield")
                              (elif (== (Variables|WallHit|GetHitWall) (Variables|WallHit|GetWall_Gym))
                                (Development|PrintString "Gym")))))))))))))))))

(fn AddSecuWallandDeactivateColl
  (Variables|WallHit|SetOneTestAtTimeSecu 2)
  (Collision|SetActorEnableCollision false))

(fn SaveAllWallsinVariables
  (bind _outactors (Actor|GetAllActorsOfClass "/Game/Room/BP_Wall.BP_Wall_C"))
  (for (_array_element _array_index) _outactors
    (switch int _array_index
      (:0
        (Variables|WallHit|SetWall_Kart _array_element))
      (:1
        (Variables|WallHit|SetWall_Judo _array_element))
      (:2
        (Variables|WallHit|SetWall_Basket _array_element))
      (:3
        (Variables|WallHit|SetWall_Tennis _array_element))
      (:4
        (Variables|WallHit|SetWall_Trackfield _array_element))
      (:5
        (Variables|WallHit|SetWall_Gym _array_element)))))

(fn ClampActorLocation
  (bind _returnvalue (Transformation|GetActorLocation))
  (Transformation|SetActorLocation (Math|Vector|MakeVector (Math|Float|Clamp(Float) (.x _returnvalue) -4.7e+03 4.7e+03) (Math|Float|Clamp(Float) (.y _returnvalue) -4.7e+03 4.7e+03) (.z _returnvalue)) false false))