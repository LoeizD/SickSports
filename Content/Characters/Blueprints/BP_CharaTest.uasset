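; BP_CharaTest is a first-person test character that moves, looks around and punches props.
; Axis inputs drive frame-time-scaled movement along control rotation, controller yaw and clamped pitch applied directly to the Camera.
; Punch runs a short object-type line trace from the Camera, with persistent debug drawing, and calls Punched on any BP_Props_Parent hit, passing the actor's forward vector.
; The construction script moves the character to a random XY position near the world origin.
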(event EventBeginPlay)

(event Input|ActionEvents|InputActionPunch
  (params (Key :type Key%20Structure :default "AnyKey"))
  (bind _camera (Variables|Default|GetCamera))
  (bind _returnvalue (Transformation|GetWorldLocation _camera))
  (:Pressed
    (bind _outhit (Collision|LineTraceForObjects _returnvalue (+ _returnvalue (* (Math|Vector|GetForwardVector _camera) 2e+02)) (Utilities|Array|MakeArray "ObjectTypeQuery7") false 0 "Persistent"))
    (bind _asbp_props_parent (Utilities|Casting|CastToBP_Props_Parent (.HitActor (Collision|BreakHitResult _outhit))))
    (Default|Punched _asbp_props_parent (Transformation|GetActorForwardVector))))

(event Input|AxisEvents|InputAxisForward
  (params (AxisValue :type Float%20%28single-precision%29))
  (Pawn|Input|AddMovementInput (Math|Vector|GetForwardVector (Pawn|GetControlRotation :!class /Script/Engine.Pawn)) (* AxisValue (* (Variables|Default|GetForwardSpeed) (Utilities|Time|GetWorldDeltaSeconds))) false))

(event Input|AxisEvents|InputAxisStrafe
  (params (AxisValue :type Float%20%28single-precision%29))
  (Pawn|Input|AddMovementInput (Math|Vector|GetRightVector (Pawn|GetControlRotation :!class /Script/Engine.Pawn)) (* AxisValue (* (Variables|Default|GetForwardSpeed) (Utilities|Time|GetWorldDeltaSeconds))) false))

(event Input|AxisEvents|InputAxisMouseUp
  (params (AxisValue :type Float%20%28single-precision%29))
  (bind _camera (Variables|Default|GetCamera))
  (Transformation|SetRelativeRotation _camera (Math|Rotator|MakeRotator 0.0 (Math|Float|Clamp(Float) (+ (.pitch (Variables|/Script/Engine.SceneComponent|GetRelativeRotation _camera)) (* AxisValue (* (Variables|Default|GetMouseSpeed) (Utilities|Time|GetWorldDeltaSeconds)))) -85.0 85.0) 0.0) false false))

(event Input|AxisEvents|InputAxisMouseRight
  (params (AxisValue :type Float%20%28single-precision%29))
  (Pawn|Input|AddControllerYawInput (* AxisValue (* (Variables|Default|GetMouseSpeed) (Utilities|Time|GetWorldDeltaSeconds)))))

(fn ConstructionScript
  (Transformation|SetActorLocation (Math|Vector|MakeVector (Math|Random|RandomFloatinRange -2e+02 2e+02) (Math|Random|RandomFloatinRange -2e+02 2e+02) 0.0) false false))