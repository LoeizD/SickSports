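; Visual motorbike rider actor that snaps to its owner pawn's BikeTarget every tick, showing the player's color and score text.
; Construction attaches bat, bunny ears, wheels and steam effect to Biker skeleton sockets.
; Tick feeds pawn inputs into a branch chain choosing animations, wheel-spin timeline, engine material parameter and steam, with debug prints; the back-left branch is disabled.
; Charge and Hit events play their own animations.
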(event Custom|Forward
  (Components|Animation|SetAnimation (Variables|Default|GetBiker) "/Game/Coco/Moto/Biker-fwd.Biker-fwd")
  (Rendering|Material|SetScalarParameterValueonMaterials (Variables|Default|GetSM_BunnyEars) "Engine" 1.0)
  (Components|Activation|SetActive (Variables|Default|GetP_Forge_SteamLeak) true false)
  (bind _newtrack_0 (Timeline|Timeline_0 Play)
    (:Update
      (Transformation|SetRelativeRotation (Variables|Default|GetRoueFront) (Math|Rotator|MakeRotator _newtrack_0 0.0 0.0) false false))))

(event Custom|Charge
  ;[1 1 1] Hit
  (Components|Animation|SetAnimation (Variables|Default|GetBiker) "/Game/Coco/Moto/NewAnimMontage2.NewAnimMontage2"))

(event Custom|Right
  (Components|Animation|SetAnimation (Variables|Default|GetBiker) "/Game/Coco/Moto/Biker-Right.Biker-Right"))

(event Custom|Hit
  ;[1 1 1] Hit
  (Components|Animation|SetAnimation (Variables|Default|GetBiker) "/Game/Coco/Moto/NewAnimMontage.NewAnimMontage"))

(event Custom|SetColor
  (params (Color :type Linear%20Color%20Structure))
  (Rendering|Material|SetVectorParameterValueonMaterials (Variables|Default|GetSM_BunnyEars) "Color" (Math|Conversions|ToVector(LinearColor) Color))
  (Rendering|Components|TextRender|SetTextRenderColor (Variables|Default|GetTextRender) (Math|Conversions|ToColor(LinearColor) Color)))

(event Custom|Movement
  (params (Fw :type Float%20%28single-precision%29) (Left :type Float%20%28single-precision%29) (Look :type Float%20%28single-precision%29))
  (bind _returnvalue (> Fw 0.0))
  (bind _returnvalue_2 (Utilities|String|ToString(Float) Look))
  (bind _returnvalue_3 (< Fw 0.0))
  (bind _returnvalue_4 (Utilities|String|ToString(Float) Fw))
  (bind _returnvalue_5 (Utilities|String|ToString(Float) Left))
  (bind _returnvalue_6 (> Left 0.0))
  (bind _returnvalue_7 (> Look 0.0))
  (bind _returnvalue_8 (Utilities|String|Append _returnvalue_4 "" _returnvalue_5 "" _returnvalue_2))
  (if (Math|Boolean|ANDBoolean _returnvalue (== Left 0.0) (== Look 0.0)) ; Forward
    (CallFunction|Forward)
    (Development|PrintString (Utilities|String|Append "Forward --- " _returnvalue_8) true true "(R=0.000000,G=0.000000,B=0.000000,A=1.000000)" 0.3)
    (elif (and _returnvalue (or (< Left 0.0) (< Look 0.0))) ; Forward Left
      (CallFunction|Forward)
      (CallFunction|Right)
      (Development|PrintString (Utilities|String|Append "Fw Right --- " _returnvalue_8) true true "(R=0.000000,G=0.000000,B=0.000000,A=1.000000)" 0.3)
      (elif (and _returnvalue (or _returnvalue_6 _returnvalue_7)) ; Forward Right
        (CallFunction|Forward)
        (CallFunction|Left)
        (Development|PrintString (Utilities|String|Append "Fw Left --- " _returnvalue_8) true true "(R=0.000000,G=0.000000,B=0.000000,A=1.000000)" 0.3)
        (elif (Math|Boolean|ANDBoolean _returnvalue_3 (== Left 0.0) (== Look 0.0)) ; Back
          (CallFunction|Back)
          (Development|PrintString (Utilities|String|Append "Back --- " _returnvalue_8) true true "(R=0.000000,G=0.000000,B=0.000000,A=1.000000)" 0.3)
          (elif (and _returnvalue_3 false) ; Back Left
            (CallFunction|Back)
            (CallFunction|Left)
            (Development|PrintString (Utilities|String|Append "Back Left--- " _returnvalue_8) true true "(R=0.000000,G=0.000000,B=0.000000,A=1.000000)" 0.3)
            (elif (and _returnvalue_3 (or _returnvalue_6 _returnvalue_7)) ; Back Right
              (CallFunction|Back)
              (CallFunction|Right)
              (Development|PrintString (Utilities|String|Append "Back Right --- " _returnvalue_8) true true "(R=0.000000,G=0.000000,B=0.000000,A=1.000000)" 0.3)
              (elif (or (< Left -0.01) (< Look -0.01)) ; Left
                (CallFunction|Left)
                (CallFunction|EngineOff)
                (Development|PrintString (Utilities|String|Append " Left--- " _returnvalue_8) true true "(R=0.000000,G=0.000000,B=0.000000,A=1.000000)" 0.3)
                (elif (or (> Left 0.01) (> Look 0.01)) ; Right
                  (CallFunction|Right)
                  (CallFunction|EngineOff)
                  (Development|PrintString (Utilities|String|Append " Right --- " _returnvalue_8) true true "(R=0.000000,G=0.000000,B=0.000000,A=1.000000)" 0.3)
                  (else
                    (CallFunction|Stop)
                    (Development|PrintString (Utilities|String|Append "STOOP --- " _returnvalue_8) true true "(R=0.000000,G=0.000000,B=0.000000,A=1.000000)" 0.3)))))))))))

(event Custom|Back
  (Components|Animation|SetAnimation (Variables|Default|GetBiker) "/Game/Coco/Moto/Biker-bwd.Biker-bwd")
  (Rendering|Material|SetScalarParameterValueonMaterials (Variables|Default|GetSM_BunnyEars) "Engine" -1.0)
  (Components|Activation|SetActive (Variables|Default|GetP_Forge_SteamLeak) true false)
  (bind _newtrack_0 (Timeline|Timeline_0 Reverse)
    (:Update
      (Transformation|SetRelativeRotation (Variables|Default|GetRoueFront) (Math|Rotator|MakeRotator _newtrack_0 0.0 0.0) false false))))

(event Custom|EngineOff
  (Rendering|Material|SetScalarParameterValueonMaterials (Variables|Default|GetSM_BunnyEars) "Engine" 0.0)
  (Components|Activation|SetActive (Variables|Default|GetP_Forge_SteamLeak) false false)
  (bind _newtrack_0 (Timeline|Timeline_0 Stop)
    (:Update
      (Transformation|SetRelativeRotation (Variables|Default|GetRoueFront) (Math|Rotator|MakeRotator _newtrack_0 0.0 0.0) false false))))

(event Custom|UpdateScore
  (params (Value :type Integer))
  (Rendering|Components|TextRender|SetText (Variables|Default|GetTextRender2) (Utilities|Text|ToText(Integer) Value)))

(event Custom|Left
  (Components|Animation|SetAnimation (Variables|Default|GetBiker) "/Game/Coco/Moto/Biker-Left.Biker-Left"))

(event Custom|Stop
  (Rendering|Material|SetScalarParameterValueonMaterials (Variables|Default|GetSM_BunnyEars) "Engine" 0.0)
  (Components|Activation|SetActive (Variables|Default|GetP_Forge_SteamLeak) false false)
  (Components|Animation|SetAnimation (Variables|Default|GetBiker) "/Game/Coco/Moto/Biker-fwd.Biker-fwd")
  (bind _newtrack_0 (Timeline|Timeline_0 Stop)
    (:Update
      (Transformation|SetRelativeRotation (Variables|Default|GetRoueFront) (Math|Rotator|MakeRotator _newtrack_0 0.0 0.0) false false))))

(event EventBeginPlay
  (CallFunction|SetColor (Variables|/Game/Characters/Blueprints/BP_Pawn.BP_Pawn_C|GetMyColor (Variables|Default|GetOwnerPawn))))

(event EventTick
  (params (DeltaSeconds :type Float%20%28single-precision%29))
  (bind _ownerpawn (Variables|Default|GetOwnerPawn))
  (bind _ownerpawn_2 (Variables|Default|GetOwnerPawn))
  (bind _biketarget (Variables|/Game/Characters/Blueprints/BP_Pawn.BP_Pawn_C|GetBikeTarget _ownerpawn))
  (bind _returnvalue (Transformation|GetWorldTransform _biketarget))
  (Transformation|SetActorLocationAndRotation (.location _returnvalue) (.rotation _returnvalue))
  (CallFunction|Movement (Variables|/Game/Characters/Blueprints/BP_Pawn.BP_Pawn_C|GetForward _ownerpawn_2) (Variables|/Game/Characters/Blueprints/BP_Pawn.BP_Pawn_C|GetLeft _ownerpawn_2) (Variables|/Game/Characters/Blueprints/BP_Pawn.BP_Pawn_C|GetLook _ownerpawn_2)))

(fn ConstructionScript
  (Transformation|AttachComponentToComponent (Variables|Default|GetBat-Only) (Variables|Default|GetBiker) "r_arm_WristSHJnt" "KeepRelative" "KeepRelative" "KeepRelative" true)
  (Transformation|AttachComponentToComponent (Variables|Default|GetSM_BunnyEars) (Variables|Default|GetBiker) "head_TopSHJnt" "KeepRelative" "KeepRelative" "KeepRelative" true)
  (Transformation|AttachComponentToComponent (Variables|Default|GetRoueFront) (Variables|Default|GetBiker) "Fork_AuxSHJnt" "KeepWorld" "KeepWorld" "KeepRelative" true)
  (Transformation|AttachComponentToComponent (Variables|Default|GetRoueBack) (Variables|Default|GetBiker) "Moto_AuxSHJnt" "KeepWorld" "KeepWorld" "KeepRelative" true)
  (Transformation|AttachComponentToComponent (Variables|Default|GetP_Forge_SteamLeak) (Variables|Default|GetBiker) "Moto_AuxSHJnt" "KeepWorld" "KeepWorld" "KeepRelative" true)
  (Transformation|AttachComponentToComponent (Variables|Default|GetScene) (Variables|Default|GetBiker) "Moto_AuxSHJnt" "KeepWorld" "KeepWorld" "KeepRelative" true))