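; Parent Blueprint for punchable props that glide across BP_Wall surfaces, taking their puncher's color through an overridable event.
; Punches add clamped speed and set direction, reversing it if the puncher is on another surface; Tick moves the prop and spins its visual.
; On authority, new wall overlaps trigger a trace and reference-frame rotations to remap the prop onto that wall, then push the transform.
; A brief collision shutoff prevents repeated transitions.
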(event OnComponentBeginOverlap(SlideOnWallsCollider)
  (params (OverlappedComponent :type Primitive%20Component%20Object%20Reference) (OtherActor :type Actor%20Object%20Reference) (OtherComp :type Primitive%20Component%20Object%20Reference) (OtherBodyIndex :type Integer) (bFromSweep :type Boolean) (SweepResult :type Hit%20Result%20Structure%20%28by%20ref%29))
  (bind _propnewdirection (Variables|Default|GetPropNewDirection))
  (bind _arrow (Variables|Default|GetArrow))
  (bind _arrow_2 (Variables|Default|GetArrow))
  (bind _returnvalue (Transformation|GetWorldRotation _propnewdirection))
  ;[0.4692 0 1] server
  (Networking|SwitchHasAuthority
    (:Authority
      (bind _asbp_wall (Utilities|Casting|CastToBP_Wall OtherActor))
      (Variables|WallHit|SetHitWall _asbp_wall)
      ;[1 1 1] Test si c'est bien un nouveau wall
      (if (and (!= (Variables|WallHit|GetHitWall) (Variables|WallHit|GetCurrentWall)) (!= (Variables|WallHit|GetHitWall) (Variables|WallHit|GetPreviousWall)))
        (if (== (Variables|WallHit|GetOneTestAtTimeSecu) 0)
          (CallFunction|AddSecuWallandDeactivateColl)
          (Variables|WallHit|SetPREPreviousWall (Variables|WallHit|GetPreviousWall))
          (Variables|WallHit|SetPreviousWall (Variables|WallHit|GetCurrentWall))
          (Variables|WallHit|SetCurrentWall (Variables|WallHit|GetHitWall))
          (Variables|Default|SetLTNormal (Math|Vector|GetForwardVector (Variables|/Game/Room/BP_Wall.BP_Wall_C|GetWallUp (Variables|WallHit|GetHitWall))))
          (CallFunction|CreateAddOfWallstoIgnore)
          (bind (_outhit _returnvalue_2) (Collision|LineTraceForObjects (+ (Transformation|GetWorldLocation _arrow) (* (Math|Vector|GetForwardVector _arrow) -3e+04)) (+ (Transformation|GetWorldLocation _arrow) (* (Math|Vector|GetForwardVector _arrow) 2e+03)) (Utilities|Array|MakeArray "ObjectTypeQuery8") false (Variables|WallHit|GetWallsToIgnore) "None"))
          (if _returnvalue_2
            (Variables|Default|SetLTImpactPoint (.ImpactPoint (Collision|BreakHitResult _outhit)))
            (Transformation|SetWorldRotation (Variables|Default|GetRepereSol) (Math|Rotator|MakeRotfromZX (Math|Vector|GetUpVector (Variables|Default|GetArrow)) (* (Variables|Default|GetLTNormal) -1.0)) false false)
            (Transformation|SetWorldRotation (Variables|Default|GetPropDirection) (Math|Rotator|MakeRotfromZX (Math|Vector|GetUpVector _arrow_2) (Math|Vector|GetForwardVector _arrow_2)) false false)
            (Transformation|SetWorldRotation (Variables|Default|GetRepereMur) (Math|Rotator|MakeRotfromZX (Variables|Default|GetLTNormal) (Math|Vector|GetUpVector (Variables|Default|GetArrow))) false false)
            (Transformation|SetRelativeRotation (Variables|Default|GetPropNewDirection) (Variables|/Script/Engine.SceneComponent|GetRelativeRotation (Variables|Default|GetPropDirection)) false false)
            (Transformation|SetActorRotation _returnvalue)
            (Transformation|SetWorldRotation (Variables|Default|GetArrow) _returnvalue false false)
            (Transformation|SetActorLocation (Variables|Default|GetLTImpactPoint) false false)
            ;[1 1 1] ToAll Update Transform
            (CallFunction|ServerUpdateTransform (Transformation|GetActorTransform) (Transformation|GetWorldRotation (Variables|Default|GetArrow)))))))))

(event Custom|Punched
  (params (PunchNewDirection :type Vector) (AddedForce :type Float%20%28single-precision%29) (OwnerCurrentFloor :type Actor%20Object%20Reference) (OwnerColor :type Linear%20Color%20Structure) (OwnerPlayer :type Actor%20Object%20Reference))
  (bind _currentwall (Variables|WallHit|GetCurrentWall))
  (bind _arrow (Variables|Default|GetArrow))
  ;[1 1 1] si besoin
  (Variables|Default|SetMyOwnerColor OwnerColor)
  (Variables|Default|SetMyOwnerPlayer OwnerPlayer)
  (CallFunction|ChangeOwnerColor OwnerColor)
  (CallFunction|HitSound)
  (if (!= (Variables|WallHit|GetCurrentWall) OwnerCurrentFloor) ; Si on n'est pas sur le même plan\nque le props qu'on tape
    ;[1 1 1] Just Reverse Arrow
    (Transformation|SetWorldRotation _arrow (Math|Rotator|MakeRotfromZX (Math|Vector|GetUpVector _arrow) (* (Math|Vector|GetForwardVector _arrow) -1.0)) false false)
    (else
      ;[1 1 1] Set arrow (so linetrace) rot
      (Transformation|SetWorldRotation (Variables|Default|GetArrow) (Math|Rotator|MakeRotfromXZ PunchNewDirection (Transformation|GetActorUpVector)) false false)))
  (Variables|Default|SetForwardVector (Math|Vector|GetForwardVector (Variables|Default|GetArrow)))
  (Variables|Movement|SetSpeed_Current (Math|Float|Clamp(Float) (+ (select (Variables|Default|GetIsPunched) (Variables|Movement|GetSpeed_Current) (Variables|Movement|GetMinSpeed)) AddedForce) 0.0 (Variables|Default|GetMaxSpeed)))
  ;[1 1 1] Reset Walls security
  (Variables|WallHit|SetPREPreviousWall _currentwall)
  (Variables|WallHit|SetPreviousWall _currentwall)
  (CallFunction|AddSecuWallandDeactivateColl)
  (Variables|Default|SetIsPunched true))

(event Custom|ChangeOwnerColor
  (params (PlayerColor :type Linear%20Color%20Structure))
  ;[1 1 1] Override par Coco
)

(event Custom|ServerUpdateTransform
  (params (NewTransform :type Transform%20%28by%20ref%29) (NewRotation :type Rotator))
  ;[1 1 1] ToAll Update Transform
  (CallFunction|UpdateMyTranform NewTransform)
  (CallFunction|SetArrowWorldRotation NewRotation))

(event EventBeginPlay
  (Class|SceneComponent|DetachfromParent (Variables|Default|GetRepereSol) false true)
  (bind (_outhit _returnvalue) (Collision|LineTraceForObjects (+ (Transformation|GetActorLocation) (* (Transformation|GetActorUpVector) 2e+01)) (+ (Transformation|GetActorLocation) (* (Transformation|GetActorUpVector) -2e+01)) (Utilities|Array|MakeArray "ObjectTypeQuery8") false 0 "None"))
  (if _returnvalue
    (Variables|WallHit|SetCurrentWall (.HitActor (Collision|BreakHitResult _outhit)))
    (Variables|WallHit|SetPreviousWall (.HitActor (Collision|BreakHitResult _outhit)))
    (Variables|WallHit|SetPREPreviousWall (.HitActor (Collision|BreakHitResult _outhit)))))

(event EventTick
  (params (DeltaSeconds :type Float%20%28single-precision%29))
  (bind _returnvalue (Transformation|GetActorLocation))
  (if (Variables|Default|GetIsPunched)
    (Utilities|FlowControl|Sequence
      (:then_0
        ;[1 1 1] Movement
        (Transformation|AddActorWorldOffset (* (* (Math|Vector|GetForwardVector (Variables|Default|GetArrow)) (Variables|Movement|GetSpeed_Current)) (Utilities|Time|GetWorldDeltaSeconds)))
        ;[1 1 1] Visual Rotation
        (Transformation|AddRelativeRotation (Variables|Default|GetVisual) (Math|Rotator|MakeRotator 0.0 0.0 (* (Math|Curves|GetFloatValue (Variables|Movement|GetCRV_RotationBySpeed) (Math|Float|Clamp(Float) (/ (Variables|Movement|GetSpeed_Current) (Variables|Default|GetMaxSpeed)))) (Variables|Movement|GetMaxVisualRotation) (Utilities|Time|GetWorldDeltaSeconds))) false false)
        ;[0 0.9182 1] log
        (if (Math|Boolean|ORBoolean (< (.x _returnvalue) -1e+04) (> (.x _returnvalue) 1e+04) (< (.y _returnvalue) -1e+04) (> (.y _returnvalue) 1e+04) (< (.z _returnvalue) -1e+04) (> (.z _returnvalue) 1e+04))
          (Development|PrintString (Utilities|String|Append "I'm OUT ! and I'm: " (Utilities|GetDisplayName self)) true true "(R=1.000000,G=1.000000,B=1.000000,A=1.000000)" 999.0)))
      (:then_1
        ;[1 1 1] Reset col secu
        (if (!= (Variables|WallHit|GetOneTestAtTimeSecu) 0)
          (bind _output_get (Variables|WallHit|SetOneTestAtTimeSecu (- (Variables|WallHit|GetOneTestAtTimeSecu) 1)))
          (if (== _output_get 0)
            (Collision|SetActorEnableCollision true)))))))

(fn ConstructionScript)

(fn UpdateMyTranform
  (params (NewTransform :type Transform%20%28by%20ref%29))
  (Transformation|SetActorTransform NewTransform))

(fn Stop
  (Variables|Default|SetIsPunched false)
  (Variables|Movement|SetSpeed_Current 0.0)
  (Variables|Default|SetMyOwnerPlayer 0))

(fn HitSound
  (bind _propsound (Variables|Default|GetPropSound))
  (bind _hitprops (Variables|Default|GetHitProps))
  (Class|FMODAudioComponent|Play _hitprops)
  (Class|FMODAudioComponent|SetParameter _hitprops "MAT" (Math|Conversions|ToFloat(Integer) (Math|Float|Floor (Math|Random|RandomFloatinRange 0.0 2.0))))
  (Class|FMODAudioComponent|Play _propsound)
  (Class|FMODAudioComponent|SetVolume _propsound 0.5))

(fn SetArrowWorldRotation
  (params (NewRotation :type Rotator))
  (Transformation|SetWorldRotation (Variables|Default|GetArrow) NewRotation false false))

(fn AddSecuWallandDeactivateColl
  (Variables|WallHit|SetOneTestAtTimeSecu 2)
  (Collision|SetActorEnableCollision false))

(fn CreateAddOfWallstoIgnore
  (Utilities|Array|Clear (Variables|WallHit|GetWallsToIgnore))
  (bind _outactors (Actor|GetAllActorsOfClass "/Game/Room/BP_Wall.BP_Wall_C"))
  (for _array_element _outactors
    (if (!= _array_element (Variables|WallHit|GetCurrentWall)) ; Si est n'importe quel wall\nsauf le wall qu'on collisionne\nsur lequel on a envie de grimper
      (Utilities|Array|Add (Variables|WallHit|GetWallsToIgnore) _array_element))))