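; BP_Jump is a prop actor, apparently a jump pad or similar jump element, whose color can be set to match an owning player.
; A ChangeOwnerColor event converts the given player color to a vector and writes it to the Color material parameter on three static mesh components.
; BeginPlay, overlap and Tick are disabled stubs, so the Blueprint contains no jump behavior of its own.
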(event EventBeginPlay
  (|CallParentFunction))

(event Collision|EventActorBeginOverlap
  (params (OtherActor :type Actor%20Object%20Reference)))

(event EventChangeOwnerColor
  (params (PlayerColor :type Linear%20Color%20Structure))
  (Rendering|Material|SetVectorParameterValueonMaterials (Variables|Default|GetStaticMesh1) "Color" (Math|Conversions|ToVector(LinearColor) PlayerColor)))

(event EventTick
  (params (DeltaSeconds :type Float%20%28single-precision%29))
  (|CallParentFunction 0.0))

(fn ConstructionScript
  (|CallParentFunction))