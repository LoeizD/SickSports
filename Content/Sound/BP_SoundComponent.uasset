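; BP_SoundComponent is an actor that plays one character's sound effects: klaxon, punch, being hit and point earned.
; BeginPlay randomizes the klaxon's Player parameter, and other events trigger each sound, with a PUNCH parameter separating hits from misses.
; Being hit plays the impact, then a voice after a short random delay.
; Every tenth klaxon calls EyesOfTiger on BP_SoundManager, and each press prints the running count.
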(event Custom|KlaxonEvent
  ;[1 1 1] Klaxon
  (Class|FMODAudioComponent|Play (Variables|Default|GetKlaxon))
  (Variables|Default|SetKlaxonPlayed (+ (Variables|Default|GetKlaxonPlayed) 1))
  (Development|PrintString (Utilities|String|ToString(Integer) (Variables|Default|GetKlaxonPlayed)))
  (if (and (== (Math|Integer|%(Integer) (Variables|Default|GetKlaxonPlayed) 10) 0) (!= (Variables|Default|GetKlaxonPlayed) 0))
    (bind _outactors (Actor|GetAllActorsOfClass "/Game/Sound/BP_SoundManager.BP_SoundManager_C"))
    (Default|EyesOfTiger _outactors)))

(event Custom|PointEarn
  ;[1 1 1] Point Earned
  (Class|FMODAudioComponent|Play (Variables|Default|GetPoint)))

(event Custom|Punch
  (params (Hit :type Boolean))
  (bind _punchsound (Variables|Default|GetPunchSound))
  ;[1 1 1] Punch
  (if Hit
    (Variables|Default|SetHitParam 1.0)
    (else
      (Variables|Default|SetHitParam 0.0)))
  (Class|FMODAudioComponent|SetParameter _punchsound "PUNCH" (Variables|Default|GetHitParam))
  (Class|FMODAudioComponent|Play _punchsound))

(event Custom|Hit
  ;[1 1 1] Being Hit
  (Class|FMODAudioComponent|Play (Variables|Default|GetHitSound))
  (Utilities|FlowControl|Delay (Math|Random|RandomFloatinRange 0.03 0.2))
  (Class|FMODAudioComponent|Play (Variables|Default|GetHitVoice)))

(event EventBeginPlay
  (Class|FMODAudioComponent|SetParameter (Variables|Default|GetKlaxon) "Player" (Math|Conversions|ToFloat(Integer) (Math|Float|Truncate (Math|Random|RandomFloatinRange 0.0 3.0)))))

(event Collision|EventActorBeginOverlap
  (params (OtherActor :type Actor%20Object%20Reference)))

(event EventTick
  (params (DeltaSeconds :type Float%20%28single-precision%29)))

(fn ConstructionScript)