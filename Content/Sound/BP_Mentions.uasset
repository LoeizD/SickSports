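; BP_Mentions plays spoken or audio "mentions" through the MentionsSound component, selecting the type by sound parameter.
; BeginPlay sets a random whole-number RAND parameter, debug-prints a separately rolled value, then fires MentionBegin.
; PointScore, MentionBegin and Mention each set ParamVar to their own value, then share one path that writes the Mentions parameter and plays the sound.
; TEst triggers the same path as Mention.
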(event Custom|PointScore
  (bind _mentionssound (Variables|Default|GetMentionsSound))
  (Variables|Default|SetParamVar 1.0)
  (Class|FMODAudioComponent|SetParameter _mentionssound "Mentions" (Variables|Default|GetParamVar))
  (Class|FMODAudioComponent|Play _mentionssound))

(event Custom|TEst
  (bind _mentionssound (Variables|Default|GetMentionsSound))
  (Variables|Default|SetParamVar 0.0)
  (Class|FMODAudioComponent|SetParameter _mentionssound "Mentions" (Variables|Default|GetParamVar))
  (Class|FMODAudioComponent|Play _mentionssound))

(event Custom|Mention%20Begin
  (bind _mentionssound (Variables|Default|GetMentionsSound))
  (Variables|Default|SetParamVar 2.0)
  (Class|FMODAudioComponent|SetParameter _mentionssound "Mentions" (Variables|Default|GetParamVar))
  (Class|FMODAudioComponent|Play _mentionssound))

(event Custom|Mention
  (bind _mentionssound (Variables|Default|GetMentionsSound))
  (Variables|Default|SetParamVar 0.0)
  (Class|FMODAudioComponent|SetParameter _mentionssound "Mentions" (Variables|Default|GetParamVar))
  (Class|FMODAudioComponent|Play _mentionssound))

(event EventBeginPlay
  (bind _returnvalue (Math|Random|RandomFloatinRange 0.0 2.0))
  (bind _returnvalue_2 (Math|Float|Truncate _returnvalue))
  (bind _returnvalue_3 (Math|Conversions|ToFloat(Integer) _returnvalue_2))
  (Development|PrintString (Utilities|String|ToString(Float) _returnvalue_3))
  (Class|FMODAudioComponent|SetParameter (Variables|Default|GetMentionsSound) "RAND" _returnvalue_3)
  (CallFunction|MentionBegin))

(event EventTick
  (params (DeltaSeconds :type Float%20%28single-precision%29)))

(fn ConstructionScript)