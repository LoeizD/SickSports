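; Sound manager that starts the game's adaptive music on BeginPlay if enabled and varies its arrangement during playback.
; Timeline beat and marker callbacks make weighted random changes to the PART parameter, with selected bars also setting PROG.
; The first variation at bar 16 enables the Cut and Break marker switches.
; EyesOfTiger selects a special part based on whether it has played, and EndTigger markers randomly move the music on.
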(event OnTimelineMarker(Music)
  (params (Name :type String) (Position :type Integer))
  (bind _returnvalue (Math|Random|RandomBoolwithWeight 0.3))
  (bind _musichasplayed (Variables|Default|GetMusicHasPlayed))
  (bind _music (Variables|Default|GetMusic))
  (CallFunction|TiggerEvent Name)
  (if (Utilities|Enum|Equal(Enum) Name "Cut")
    (if _musichasplayed
      (if (Math|Random|RandomBoolwithWeight 0.8)
        (Class|FMODAudioComponent|SetParameter _music "PART" (Math|Conversions|ToFloat(Integer) (Math|Float|Floor (Math|Random|RandomFloatinRange 1.0 5.0))))))
    (elif (and (Utilities|Enum|Equal(Enum) Name "Break") _musichasplayed)
      (if _returnvalue
        (Class|FMODAudioComponent|SetParameter _music "PART" 5.0))
      (elif _returnvalue
        (if (Utilities|Enum|Equal(Enum) Name "EndTigger")
          (Variables|Default|SetTigerPlayed true)
          (Class|FMODAudioComponent|SetParameter _music "PART" (Math|Conversions|ToFloat(Integer) (Math|Float|Floor (Math|Random|RandomFloatinRange 1.0 5.0)))))))))

(event OnTimelineBeat(Music)
  (params (Bar :type Integer) (Beat :type Integer) (Position :type Integer) (Tempo :type Float%20%28single-precision%29) (TimeSignatureUpper :type Integer) (TimeSignatureLower :type Integer))
  (bind _music (Variables|Default|GetMusic))
  (bind _music_2 (Variables|Default|GetMusic))
  (if (== Bar 16)
    (Class|FMODAudioComponent|SetParameter _music "PART" (Math|Conversions|ToFloat(Integer) (Math|Float|Floor (Math|Random|RandomFloatinRange 1.0 5.0))))
    (Utilities|FlowControl|Delay 2.0)
    (Class|FMODAudioComponent|SetParameter _music "PROG" (Variables|Default|GetMusicProg))
    (Variables|Default|SetMusicProg 2.0)
    (Variables|Default|SetMusicHasPlayed true)
    (elif (Math|Boolean|ORBoolean (== Bar 24) (== Bar 28) (== Bar 40) (== Bar 32))
      (if (Math|Random|RandomBoolwithWeight 0.8)
        (Class|FMODAudioComponent|SetParameter _music_2 "PART" (Math|Conversions|ToFloat(Integer) (Math|Float|Floor (Math|Random|RandomFloatinRange 0.0 5.0))))
        (if (Math|Random|RandomBoolwithWeight 0.3)
          (Class|FMODAudioComponent|SetParameter _music_2 "PROG" 2.0)
          (else
            (Class|FMODAudioComponent|SetParameter _music_2 "PROG" 1.0)))))))

(event Custom|EyesOfTiger
  (bind _music (Variables|Default|GetMusic))
  (if (Variables|Default|GetTigerPlayed)
    (Class|FMODAudioComponent|SetParameter _music "PART" 7.0)
    (else
      (Class|FMODAudioComponent|SetParameter _music "PART" 6.0))))

(event Custom|TiggerEvent
  (params (Name :type String))
  (if (Utilities|Enum|Equal(Enum) Name "EndTigger")
    (if (Math|Random|RandomBoolwithWeight 0.9)
      (Class|FMODAudioComponent|SetParameter (Variables|Default|GetMusic) "PART" 0.0))))

(event EventBeginPlay
  (if (Variables|Default|GetMusicOn)
    (Class|FMODAudioComponent|Play (Variables|Default|GetMusic))))

(event Input|KeyboardEvents|J
  (params (Key :type Key%20Structure :default "AnyKey")))

(fn ConstructionScript)