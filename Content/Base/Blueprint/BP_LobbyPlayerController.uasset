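; Lobby player controller that shows the lobby UI and relays host and join requests to the game instance.
; On BeginPlay it creates and displays UI_Lobby, switches to game-and-UI input focused on it, and shows the mouse cursor.
; Its host and join events cast to BP_GameInstance and pass the controller, plus search text when joining, to its session functions.
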(event Custom|Player_Server_HostLobby
  (bind _asbp_game_instance (Utilities|Casting|CastToBP_GameInstance (Game|GetGameInstance)))
  (Default|InstanceLobby _asbp_game_instance self))

(event Custom|JoinParty
  (params (Txt_Search :type Text%20Block%20Object%20Reference))
  (bind _asbp_game_instance (Utilities|Casting|CastToBP_GameInstance (Game|GetGameInstance)))
  (Default|JointheSession _asbp_game_instance self Txt_Search))

(event EventBeginPlay
  (bind _returnvalue (UserInterface|CreateWidget "/Game/UI/UI_Lobby.UI_Lobby_C"))
  (bind _output_get (Variables|Default|SetUI_Lobby_REF _returnvalue))
  (UserInterface|Viewport|AddtoViewport _output_get 0)
  (Input|SetInputModeGameandUI self _output_get "DoNotLock" true)
  (Variables|Default|SetbShowMouseCursor true))

(fn ConstructionScript)