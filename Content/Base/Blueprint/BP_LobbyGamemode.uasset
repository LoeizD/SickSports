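; Lobby game mode that handles the lobby's opening audio: a mentions sound followed by music.
; On BeginPlay it sets the MentionsSound RAND parameter, sets Mentions to a fixed value, plays it, then starts the MUSIC event in 2D after a short delay.
; RAND comes from truncating a random float between zero and one, so it is effectively always zero.
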(event Custom|Mention%20Begin
  (bind _mentionssound (Variables|Default|GetMentionsSound))
  (bind _output_get (Variables|Default|SetParamVar 2.0))
  (Class|FMODAudioComponent|SetParameter _mentionssound "Mentions" _output_get)
  (Class|FMODAudioComponent|Play _mentionssound))

(event EventBeginPlay
  (Class|FMODAudioComponent|SetParameter (Variables|Default|GetMentionsSound) "RAND" (Math|Conversions|ToFloat(Integer) (Math|Float|Truncate (Math|Random|RandomFloatinRange 0.0 1.0))))
  (CallFunction|MentionBegin)
  (Utilities|FlowControl|Delay 1.5)
  (Class|FMODBlueprintStatics|PlayEvent2D "/Game/FMOD/Events/MUSIC.MUSIC"))

(fn ConstructionScript)